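; SaveGame object that persists a run's state: seeds, tile and sector map data, planets, crew, ship, cargo, upgrades and scrap.
; SaveAllData copies these fields from a passed-in savable object, then writes itself to the SaveName slot; its AddSaveSlot branch is empty.
; LoadAllData copies the stored fields back onto a valid target object, printing a failure message otherwise, and does no slot reading itself.
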(fn SaveAllData
  (params (SavableObj :type Game%20Inst%20BP%20Object%20Reference) (AddSaveSlot? :type Boolean))
  (Utilities|FlowControl|Sequence
    (:then_0
      (Variables|Default|SetGameSeedStream (Variables|/Game/AllLevelContent/GameInst_BP.GameInst_BP_C|GetGameSeedStream SavableObj))
      (Variables|Default|SetGame%20Seed%20Known%20Int (Variables|/Game/AllLevelContent/GameInst_BP.GameInst_BP_C|GetGameSeedKnownInt SavableObj))
      (Variables|Default|SetTile%20Seed%20Ints (Variables|/Game/AllLevelContent/GameInst_BP.GameInst_BP_C|GetTileSeedInts SavableObj))
      (Variables|Default|SetLast%20Tile%20Int (Variables|/Game/AllLevelContent/GameInst_BP.GameInst_BP_C|GetLastTileInt SavableObj))
      (Variables|Default|SetCurrent%20Tile%20Data (Variables|/Game/AllLevelContent/GameInst_BP.GameInst_BP_C|GetCurrentTileData SavableObj))
      (Variables|Default|SetInven%20Slot%20Content%20Cargo (Variables|/Game/AllLevelContent/GameInst_BP.GameInst_BP_C|GetInvenSlotContent_Cargo SavableObj))
      (Variables|Default|SetCrew (Variables|/Game/AllLevelContent/GameInst_BP.GameInst_BP_C|GetCrew SavableObj))
      (Variables|Default|SetShip%20Data (Variables|/Game/AllLevelContent/GameInst_BP.GameInst_BP_C|GetShipData SavableObj))
      (Variables|Default|SetScrap%20Num (Variables|/Game/AllLevelContent/GameInst_BP.GameInst_BP_C|GetScrapNum SavableObj))
      (Variables|Default|SetCurrent%20Planet%20Seed (Variables|/Game/AllLevelContent/GameInst_BP.GameInst_BP_C|GetCurrentPlanetSeed SavableObj))
      (Variables|Default|SetUsed%20Plot%20Keys (Variables|/Game/AllLevelContent/GameInst_BP.GameInst_BP_C|GetUsedPlotKeys SavableObj))
      (Variables|Default|SetUpgrades%20Inven (Variables|/Game/AllLevelContent/GameInst_BP.GameInst_BP_C|GetUpgrades_Inven SavableObj))
      (Variables|Default|SetSaved%20Planets (Variables|/Game/AllLevelContent/GameInst_BP.GameInst_BP_C|GetSavedPlanets SavableObj))
      (Variables|Default|SetVisible%20Tile%20Ints (Variables|/Game/AllLevelContent/GameInst_BP.GameInst_BP_C|GetVisibleTileInts SavableObj))
      (Variables|Default|SetSectorMapData (Variables|/Game/AllLevelContent/GameInst_BP.GameInst_BP_C|GetSectorMapData SavableObj))
      (Variables|Default|SetAllTilesData (Variables|/Game/AllLevelContent/GameInst_BP.GameInst_BP_C|GetAllTilesData SavableObj)))
    (:then_1
      (if AddSaveSlot?
        _
        (else
          _))
      (SaveGame|SaveGametoSlot self (Variables|Default|GetSaveName)))))

(fn LoadAllData
  (params (SavableObj :type Game%20Inst%20BP%20Object%20Reference))
  (Utilities|IsValid SavableObj
    (:Is%20Valid
      (Variables|/Game/AllLevelContent/GameInst_BP.GameInst_BP_C|SetGameSeedStream SavableObj (Variables|Default|GetGameSeedStream))
      (Variables|/Game/AllLevelContent/GameInst_BP.GameInst_BP_C|SetGameSeedKnownInt SavableObj (Variables|Default|GetGame%20Seed%20Known%20Int))
      (Variables|/Game/AllLevelContent/GameInst_BP.GameInst_BP_C|SetTileSeedInts SavableObj (Variables|Default|GetTile%20Seed%20Ints))
      (Variables|/Game/AllLevelContent/GameInst_BP.GameInst_BP_C|SetLastTileInt SavableObj (Variables|Default|GetLast%20Tile%20Int))
      (Variables|/Game/AllLevelContent/GameInst_BP.GameInst_BP_C|SetCurrentTileData SavableObj (Variables|Default|GetCurrent%20Tile%20Data))
      (Variables|/Game/AllLevelContent/GameInst_BP.GameInst_BP_C|SetInvenSlotContent_Cargo SavableObj (Variables|Default|GetInven%20Slot%20Content%20Cargo))
      (Variables|/Game/AllLevelContent/GameInst_BP.GameInst_BP_C|SetCrew SavableObj (Variables|Default|GetCrew))
      (Variables|/Game/AllLevelContent/GameInst_BP.GameInst_BP_C|SetShipData SavableObj (Variables|Default|GetShip%20Data))
      (Variables|/Game/AllLevelContent/GameInst_BP.GameInst_BP_C|SetScrapNum SavableObj (Variables|Default|GetScrap%20Num))
      (Variables|/Game/AllLevelContent/GameInst_BP.GameInst_BP_C|SetCurrentPlanetSeed SavableObj (Variables|Default|GetCurrent%20Planet%20Seed))
      (Variables|/Game/AllLevelContent/GameInst_BP.GameInst_BP_C|SetUsedPlotKeys SavableObj (Variables|Default|GetUsed%20Plot%20Keys))
      (Variables|/Game/AllLevelContent/GameInst_BP.GameInst_BP_C|SetUpgrades_Inven SavableObj (Variables|Default|GetUpgrades%20Inven))
      (Variables|/Game/AllLevelContent/GameInst_BP.GameInst_BP_C|SetSavedPlanets SavableObj (Variables|Default|GetSaved%20Planets))
      (Variables|/Game/AllLevelContent/GameInst_BP.GameInst_BP_C|SetVisibleTileInts SavableObj (Variables|Default|GetVisible%20Tile%20Ints))
      (Variables|/Game/AllLevelContent/GameInst_BP.GameInst_BP_C|SetSectorMapData SavableObj (Variables|Default|GetSectorMapData))
      (Variables|/Game/AllLevelContent/GameInst_BP.GameInst_BP_C|SetAllTilesData SavableObj (Variables|Default|GetAllTilesData)))
    (:Is%20Not%20Valid
      (Development|PrintString 0 "FAILURE TO GET LOAD" true true "(R=0.255393,G=0.000000,B=1.000000,A=1.000000)"))))