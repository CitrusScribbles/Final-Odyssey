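; Game instance that holds persistent game state: save object, seeded random stream, cargo inventory, crew and music.
; Init creates the save object early so menus get a valid reference.
; BeginAgain starts a run by applying the seed, resetting cargo to starter items, picking a preset crew and saving.
; SetMusic crossfades songs through one MetaSound, using a watched playback-time output to resume the transition at the correct position.
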(event Custom|BeginAgain
  ;[0 0 0 0.5] Setting up the game
  (CallFunction|SetGameSeed)
  (CallFunction|SetCargoEmpty)
  (CallFunction|PickCrew (Utilities|Array|MakeArray "NewEnumerator4" "NewEnumerator0" "NewEnumerator6" "NewEnumerator2") (Variables|Ship|GetCrew))
  (bind _hassave_ (CallFunction|CheckifSave))
  (CallFunction|SaveGame _hassave_))

(event Custom|SetMusic
  (params (NewSong :type Sound%20Wave%20Object%20Reference) (OldSong :type Sound%20Wave%20Object%20Reference))
  ;[0 0 0 0.5] Music
  ;;[0.15 0.15 0.15 0.5] Music holder and transition
  (Variables|Music|SetSong NewSong)
  (if (!= NewSong OldSong)
    (Utilities|IsValid (Variables|Default|GetMusicConductor_Ref)
      (:Is%20Valid
        (Class|AudioComponent|SetWaveParameter (Variables|Default|GetMusicConductor_Ref) "NewMusic" NewSong)
        (Class|AudioComponent|SetWaveParameter (Variables|Default|GetMusicConductor_Ref) "OldMusic" OldSong)
        (Utilities|FlowControl|Sequence
          (:then_0
            ;;[0.15 0.15 0.15 0.5] Tracking location of the song so that the music starts in the correct place.
            (MetaSoundOutput|WatchOutput (WorldSubsystems|GetMetaSoundOutputSubsystem) (Variables|Default|GetMusicConductor_Ref) "OldMusicTime" (delegate Custom|MusicTimer) "None" "None" :!class /Script/MetasoundEngine.MetaSoundOutputSubsystem :!label _label))
          (:then_1
            (bind _output_get (Variables|Default|SetMusicTimeStamp (Variables|Default|GetTempMusicTIme)))
            (Audio|Components|Audio|Play (Variables|Default|GetMusicConductor_Ref) 0.0)
            (Audio|Parameter|SetFloatParameter (Variables|Default|GetMusicConductor_Ref) "ResumeTime" (+ _output_get 0.013) :!class /Script/AudioExtensions.AudioParameterControllerInterface)
            (Class|AudioParameterControllerInterface|SetTriggerParameter (Variables|Default|GetMusicConductor_Ref) "Crossfade"))))
      (:Is%20Not%20Valid
        (bind _returnvalue (Audio|SpawnSound2D "/Game/Sound/Settings/Crossfade_Sound.Crossfade_Sound" 1.0 1.0 0.0 0 true false))
        (bind _output_get_2 (Variables|Default|SetMusicConductor_Ref _returnvalue))
        (Class|AudioComponent|SetWaveParameter _output_get_2 "OldMusic" NewSong)
        (goto _label)))))

(event Custom|MusicTimer
  (params (OutputName :type Name) (Output :type Meta%20Sound%20Output%20Structure%20%28by%20ref%29))
  ;[0 0 0 0.5] Music
  ;;[0.15 0.15 0.15 0.5] Tracking location of the song so that the music starts in the correct place.
  (bind (_success _returnvalue) (Class|MetasoundOutputBlueprintAccess|GetFloat Output))
  (if _success
    (Variables|Default|SetTempMusicTIme _returnvalue)))

(event EventInit
  ;[0 0 0 0.5] Saving
  ;;[0 0 0 0.5] Need this to happen before the menu is constructed so that the save game reference is valid.
  (bind _returnvalue (SaveGame|CreateSaveGameObject "/Game/AllLevelContent/SaveGame_BP.SaveGame_BP_C"))
  (bind _output_get (Variables|GameInfo|SetSaveGame_ref _returnvalue))
  ;;;[0.1979 0.146 0 0.5] Later have a different naming system
  (Variables|/Game/AllLevelContent/SaveGame_BP.SaveGame_BP_C|SetSaveName _output_get "UrABitch"))

(event EventSaveCargo
  ;[0 0 0 0.5] Saving
  ;;[0 0 0 0.5] Cargo
  (bind _invenitems (CallFunction|GetItems))
  (Variables|Ship|SetInvenSlotContent_Cargo _invenitems))

(fn SetGameSeed
  (Math|Random|SetRandomStreamSeed (Variables|GameInfo|GetGameSeedStream) (Variables|GameInfo|GetGameSeedKnownInt)))

(fn SetCargoEmpty
  (for _index (range 1 25)
    (Utilities|Array|SetArrayElem (Variables|Ship|GetInvenSlotContent_Cargo) (- _index 1) (Utilities|Struct|MakeStruct_InvenSlot "None" 0 false 0) true))
  ;[0.009652 0.15 0 0.5] Starting Inventory!
  (CallFunction|AddtoInven "Fuel" 3 0.0)
  (CallFunction|AddtoInven "Metal" 2 0.0)
  (CallFunction|AddtoInven "Medicine" 2 0.0))

(fn GenNewSeed
  (Variables|GameInfo|SetGameSeedKnownInt (Math|Random|RandomIntegerinRange 0 100000000))
  (CallFunction|SetGameSeed))

(fn AsGameInstance
  (return self))

(fn AsGameSave
  (return 0))

(fn GetItems
  (return 0))